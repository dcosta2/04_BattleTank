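; Player-controlled tank Blueprint that wires input to its aiming and movement components.
; On BeginPlay it hands the barrel and turret to TankAiming and both tracks to TankMovement.
; Aim axes rotate an azimuth gimbal and spring arm for the camera, while movement and fire inputs forward to those components.
; Both turn axes feed IntendTurnRight, and a Quit action exits the game.
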(event EventBeginPlay)

(event Collision|EventActorBeginOverlap
  (params (OtherActor :type Actor%20Object%20Reference)))

(event EventTick
  (params (DeltaSeconds :type Float%20%28single-precision%29)))

(event EventBeginPlay
  ;[1 1 1] Setup Tank
  (Class|TankAimingComponent|Initialise (Variables|Components|GetTankAiming) (Variables|Components|GetTankBarrel) (Variables|Components|GetTankTurret))
  (Class|TankMovementComponent|Initialise (Variables|Components|GetTankMovement) (Variables|Components|GetLeftTrack) (Variables|Components|GetRightTrack)))

(event Input|ActionEvents|InputActionQuit
  (params (Key :type Key%20Structure))
  ;[1 1 1] Quit
  (:Pressed
    (Game|QuitGame (Game|GetPlayerController 0) "Quit" false)))

(event Input|ActionEvents|InputActionFire
  (params (Key :type Key%20Structure))
  ;[1 1 1] Input Binding (Movement/Firing)
  (:Pressed
    (Class|TankAimingComponent|Fire (Variables|Components|GetTankAiming))))

(event Input|AxisEvents|InputAxisAltitude
  (params (AxisValue :type Float%20%28single-precision%29))
  ;[1 1 1] Camera Setup
  (Transformation|AddLocalRotation (Variables|Components|GetSpringArm) (Math|Rotator|MakeRotator 0.0 (* AxisValue 1.0) 0.0) false false))

(event Input|AxisEvents|InputAxisAimAzimuth
  (params (AxisValue :type Float%20%28single-precision%29))
  ;[1 1 1] Camera Setup
  (Transformation|AddLocalRotation (Variables|Components|GetAzimuthGimbal) (Math|Rotator|MakeRotator 0.0 0.0 (* AxisValue 1.0)) false false))

(event Input|AxisEvents|InputAxisTurnLeft
  (params (AxisValue :type Float%20%28single-precision%29))
  ;[1 1 1] Input Binding (Movement/Firing)
  (Class|TankMovementComponent|IntendTurnRight (Variables|Components|GetTankMovement) AxisValue))

(event Input|AxisEvents|InputAxisMoveForward
  (params (AxisValue :type Float%20%28single-precision%29))
  ;[1 1 1] Input Binding (Movement/Firing)
  (Class|TankMovementComponent|IntendMoveForward (Variables|Components|GetTankMovement) AxisValue))

(event Input|AxisEvents|InputAxisTurnRight
  (params (AxisValue :type Float%20%28single-precision%29))
  ;[1 1 1] Input Binding (Movement/Firing)
  (Class|TankMovementComponent|IntendTurnRight (Variables|Components|GetTankMovement) AxisValue))

(fn ConstructionScript)